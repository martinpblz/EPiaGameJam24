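; BP_PlayerController is a player controller intended to drive BP_Character for two local players through separate Player1 and Player2 axis inputs.
; An IsPlayer1 macro branches on whether Playerid is 0, to separate each player's shoot, obstacle and movement calls.
; That routing and the Playerid and character setup are disconnected: axis events are empty, and Possess only casts the pawn for non-Player1 controllers.
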(event `self.ReceiveBeginPlay`)

(event `self.ReceivePossess`
  (params (PossessedPawn :type "Pawn Object Reference"))
  (`self.IsPlayer1`
    (:`false`
      (cast `/Game/Players/BP_Character` PossessedPawn))))

(event `InputAction|Player2_Shoot` :consume false
  (params (Key :type "Key Structure"))
  ;[1 1 1] Player2
)

(event `InputAction|Player2_Obstacle` :consume false
  (params (Key :type "Key Structure"))
  ;[1 1 1] Player2
)

(event `InputAction|Player1_Shoot` :consume false
  (params (Key :type "Key Structure"))
  ;[1 1 1] Player1
)

(event `InputAction|Player1_Obstacle` :consume false
  (params (Key :type "Key Structure"))
  ;[1 1 1] Player1
)

(event `InputAxis|Player2_Forward` :consume false
  (params (AxisValue :type "Float (single-precision)"))
  ;[1 1 1] Player2
)

(event `InputAxis|Player1_Forward` :consume false
  (params (AxisValue :type "Float (single-precision)"))
  ;[1 1 1] Player1
)

(event `InputAxis|Player2_Vertical` :consume false
  (params (AxisValue :type "Float (single-precision)"))
  ;[1 1 1] Player2
)

(event `InputAxis|Player1_Vertical` :consume false
  (params (AxisValue :type "Float (single-precision)"))
  ;[1 1 1] Player1
)

(event `InputAxis|Player2_Horizontal` :consume false
  (params (AxisValue :type "Float (single-precision)"))
  ;[1 1 1] Player2
)

(event `InputAxis|Player1_Horizontal` :consume false
  (params (AxisValue :type "Float (single-precision)"))
  ;[1 1 1] Player1
)

(fn `UserConstructionScript`)