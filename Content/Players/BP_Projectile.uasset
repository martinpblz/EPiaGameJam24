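; Player projectile that penalizes any character it hits, other than the one who fired it.
; Each Tick it moves along its forward vector by Velocity with a swept teleport, without delta-time scaling, so speed depends on frame rate.
; Trigger overlaps with a BP_Character that is not the Instigator call Penalize on that character and destroy the projectile; other overlaps are ignored.
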(event `self.ReceiveTick`
  (params (DeltaSeconds :type "Float (single-precision)"))
  (`self.K2_SetActorLocation` (+ (`self.K2_GetActorLocation`) (* (`self.GetActorForwardVector`) (`self.Velocity`))) true true))

(event `self.Trigger.OnComponentBeginOverlap`
  (params (OverlappedComponent :type "PrimitiveComponent Object Reference") (OtherActor :type "Actor Object Reference") (OtherComp :type "PrimitiveComponent Object Reference") (OtherBodyIndex :type Integer) (bFromSweep :type Boolean) (SweepResult :type "HitResult Structure (by ref)"))
  ;[1 1 1] Check if isn't player that shooted
  (bind _asbp_character (cast `/Game/Players/BP_Character` OtherActor))
  (if (not (== _asbp_character (`self.GetInstigator`)))
    ;[1 1 1] Penalize player that got shot
    (`/Game/Players/BP_Character.Penalize` _asbp_character "NewEnumerator1")
    (`self.K2_DestroyActor`)))

(fn `UserConstructionScript`)