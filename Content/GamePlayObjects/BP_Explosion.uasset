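; BP_Explosion is a one-shot explosive prop that blows up when a BP_Character enters its TRIGGER volume.
; The first valid overlap enables gravity on its geometry collection, sets the trigger to ignore all channels and applies a strong upward impulse.
; After a short delay it spawns a scaled-up particle effect and plays an explosion sound at the actor's location.
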(event `self.TRIGGER.OnComponentBeginOverlap`
  (params (OverlappedComponent :type "PrimitiveComponent Object Reference") (OtherActor :type "Actor Object Reference") (OtherComp :type "PrimitiveComponent Object Reference") (OtherBodyIndex :type Integer) (bFromSweep :type Boolean) (SweepResult :type "HitResult Structure (by ref)"))
  (bind _returnvalue (`self.K2_GetActorLocation`))
  (bind _asbp_character (cast `/Game/Players/BP_Character` OtherActor))
  (`/Engine/EditorBlueprintResources/StandardMacros.DoOnce` false
    (:`Completed`
      (`PrimitiveComponent.SetEnableGravity` (`self.GeometryCollectionComponent`) true)
      (`PrimitiveComponent.SetCollisionResponseToAllChannels` (`self.TRIGGER`) "ECR_Ignore")
      (`PrimitiveComponent.AddImpulse` (`self.GeometryCollectionComponent`) (0.0 0.0 100000.0) "None" false)
      (`KismetSystemLibrary.Delay` 0.3)
      (`GameplayStatics.SpawnEmitterAtLocation` "/Engine/Tutorial/SubEditors/TutorialAssets/TutorialParticleSystem.TutorialParticleSystem" _returnvalue (struct) (2.0 2.0 2.0))
      (`GameplayStatics.PlaySoundAtLocation` "/Game/Assets/Music/Explo_Sion.Explo_Sion" _returnvalue (struct) 1.2 1.0 0.0 null null null null))))

(fn `UserConstructionScript`)